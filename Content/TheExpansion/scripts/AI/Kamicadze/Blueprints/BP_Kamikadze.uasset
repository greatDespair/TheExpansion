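; BP_Kamikadze is the Blueprint for an AI-controlled Kamikadze character, tagged as such on BeginPlay.
; Each tick it shows the TEEnergy energy value on a text component.
; DoAttack enables the hitbox for queries, or disables it and clears IsAttacking when the attack ends.
; On death it disables the hitbox, flags itself dead, zeroes energy, stops the AI brain logic and destroys itself after a short delay.
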(event `self.ReceiveBeginPlay`
  (`parent.ReceiveBeginPlay`)
  (`KismetArrayLibrary.Array_Add` (`self.Tags`) "Kamikadze"))

(event `self.ReceiveTick`
  (params (DeltaSeconds :type "Float (single-precision)"))
  (`parent.ReceiveTick` DeltaSeconds)
  (`TextRenderComponent.K2_SetText` (`self.EnergyTextComponent`) (`KismetTextLibrary.Conv_DoubleToText` (`TEEnergyComponent.Energy` (`self.TEEnergy`)) "HalfToEven")))

(event `self.OnDeath`
  (`PrimitiveComponent.SetCollisionEnabled` (`self.Hitbox`) "NoCollision")
  (set `self.IsDead` true)
  (set `TEEnergyComponent.Energy` 0.0 (`self.TEEnergy`))
  (`BrainComponent.StopLogic` (`AIController.BrainComponent` (`AIBlueprintHelperLibrary.GetAIController` self)) "")
  (`KismetSystemLibrary.Delay` 1.5)
  (`self.K2_DestroyActor`))

(event `self.doAttack`
  (params (isAttack :type Boolean))
  (bind _hitbox (`self.Hitbox`))
  (if isAttack
    (`PrimitiveComponent.SetCollisionEnabled` _hitbox "QueryOnly")
    (else
      (`PrimitiveComponent.SetCollisionEnabled` _hitbox "NoCollision")
      (set `self.IsAttacking` false))))

(fn `UserConstructionScript`
  (`parent.UserConstructionScript`))