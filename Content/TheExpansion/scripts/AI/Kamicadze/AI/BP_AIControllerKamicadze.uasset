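; AI controller for the Kamicadze enemy that starts its behavior tree on BeginPlay.
; When perception updates and the blackboard has no valid Enemy, it scans the updated actors for a target.
; It stores the first living AIClass actor or any BP_TEBaseRobot as Enemy, with no death check for robots.
; An existing valid Enemy is never replaced here.
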(event `self.ReceiveBeginPlay`
  (`self.RunBehaviorTree` "/Game/TheExpansion/scripts/AI/Kamicadze/AI/BT_AIKamicadze.BT_AIKamicadze"))

(event `self.AIPerception.OnPerceptionUpdated`
  (params (UpdatedActors :type "Array of Actor Object Reference (by ref)"))
  (bind _returnvalue (`AIBlueprintHelperLibrary.GetBlackboard` null))
  (`/Engine/EditorBlueprintResources/StandardMacros.IsValid` (`BlackboardComponent.GetValueAsObject` _returnvalue "Enemy")
    (:`Is Not Valid`
      (for _array_element UpdatedActors
        (bind _asaiclass (cast `/Game/TheExpansion/scripts/AI/AIClass` _array_element)
          (:`then`
            (if (not (`/Game/TheExpansion/scripts/AI/AIClass.IsDead` _asaiclass))
              (`BlackboardComponent.SetValueAsObject` _returnvalue "Enemy" _asaiclass)
              (break)))
          (:`CastFailed`
            (bind _asbp_tebase_robot (cast `/Game/TheExpansion/BP_TERobot/BP_TEBaseRobot` _array_element))
            (`BlackboardComponent.SetValueAsObject` _returnvalue "Enemy" _asbp_tebase_robot)
            (break)))))))

(fn `UserConstructionScript`)