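; BP_MeshMain is a pickup item actor with a name label that turns to face the player.
; BeginPlay fills and hides the widget text; ShowText reveals it and starts a looping timer updating its yaw, which HiddenText clears.
; Interaction records the item's class in BP_TEBaseRobot's parallel inventory and count arrays, then destroys the actor.
; Repeat pickups set that item's count from the first slot's count plus one, not its own.
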(event `Using`)

(event `HiddenText`
  (`Widget.SetVisibility` (`self.TextObj`) "Hidden")
  (`KismetSystemLibrary.K2_ClearAndInvalidateTimerHandle` (stale `ShowText` _returnvalue)))

(event `self.ReceiveBeginPlay`
  (bind _asobject_name (cast `/Game/TheExpansion/inventory/widget/ObjectName` (`WidgetComponent.GetUserWidgetObject` (`self.Widget`))))
  (bind _nameobject (`/Game/TheExpansion/inventory/widget/ObjectName.NaMeObject` _asobject_name))
  (`TextBlock.SetText` _nameobject (`self.name`))
  (set `self.TextObj` _nameobject)
  (`self.HiddenText`))

(event `ShowText`
  (`Widget.SetVisibility` (`/Game/TheExpansion/inventory/widget/ObjectName.NaMeObject` (stale `self.ReceiveBeginPlay` _asobject_name)) "Visible")
  (bind _returnvalue (`KismetSystemLibrary.K2_SetTimerDelegate` (delegate `RotateText`) 0.05 true)))

(event `RotateText`
  (bind _widget (`self.Widget`))
  (bind (_returnvalue_roll _returnvalue_pitch _returnvalue_yaw) (`KismetMathLibrary.BreakRotator` (`KismetMathLibrary.FindLookAtRotation` (`SceneComponent.K2_GetComponentLocation` _widget) (`self.K2_GetActorLocation` (`GameplayStatics.GetPlayerCharacter` 0)))))
  (`SceneComponent.K2_SetWorldRotation` _widget (`KismetMathLibrary.MakeRotator` 0.0 0.0 _returnvalue_yaw) false false))

(event `/Game/TheExpansion/inventory/Mesh/Interaction.Interaction`
  (bind _returnvalue (`GameplayStatics.GetObjectClass` self))
  ;[1 1 1] Отображение подобранных предметов в инвентаре и уничтожение их
  (bind _asbp_tebase_robot (cast `/Game/TheExpansion/BP_TERobot/BP_TEBaseRobot` (`GameplayStatics.GetPlayerCharacter` 0)))
  (bind _inventory_var (`/Game/TheExpansion/BP_TERobot/BP_TEBaseRobot.Inventory_var` _asbp_tebase_robot))
  (if (`KismetArrayLibrary.Array_Contains` _inventory_var _returnvalue)
    (bind _inventcount (`/Game/TheExpansion/BP_TERobot/BP_TEBaseRobot.InventCount` _asbp_tebase_robot))
    (`KismetArrayLibrary.Array_Set` _inventcount (`KismetArrayLibrary.Array_Find` _inventory_var _returnvalue) (+ (`|GetArrayItem` _inventcount) 1))
    (else
      (`KismetArrayLibrary.Array_Add` _inventory_var _returnvalue)
      (`KismetArrayLibrary.Array_Add` _inventcount 1)))
  (`self.K2_DestroyActor`))

(fn `UserConstructionScript`)